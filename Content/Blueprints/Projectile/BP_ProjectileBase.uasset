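; BP_ProjectileBase is a homing projectile actor that seeks a BP_EnemyCharacter.
; On BeginPlay it searches those characters for the first with Ally set to Enemy, assigns its root component as the ProjectileMovement homing target, and zeroes the starting velocity.
; Each Tick it rotates the actor to face its direction of travel, derived from the current velocity.
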(event `self.ReceiveBeginPlay`
  (bind _projectilemovement (`self.ProjectileMovement`))
  (bind _outactors (`GameplayStatics.GetAllActorsOfClass` "/Game/Blueprints/Core/BP_EnemyCharacter.BP_EnemyCharacter_C"))
  (for _array_element _outactors
    (if (`|EnumEquality` (`/Game/Blueprints/Core/BP_Character.Ally` _array_element) "Enemy")
      (break)))
  (bind _output_get (set `self.HomingTarget` _array_element))
  (set `ProjectileMovementComponent.HomingTargetComponent` (`Actor.RootComponent` _output_get) _projectilemovement)
  (set `ProjectileMovementComponent.bIsHomingProjectile` true _projectilemovement)
  (set `MovementComponent.Velocity` (0.0 0.0 0.0) _projectilemovement))

(event `self.ReceiveActorBeginOverlap`
  (params (OtherActor :type "Actor Object Reference")))

(event `self.ReceiveTick`
  (params (DeltaSeconds :type "Float (single-precision)"))
  (bind _returnvalue (`SceneComponent.K2_GetComponentLocation` (`self.Sphere`)))
  (`self.K2_SetActorRotation` (`KismetMathLibrary.FindLookAtRotation` _returnvalue (+ _returnvalue (`self.GetVelocity`)))))

(fn `UserConstructionScript`)