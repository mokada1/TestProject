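; AI controller that drives a BP_AIPlayerCharacter pawn by replaying broadcast player input.
; Move and action messages are queued, then processed one of each per Tick while alive, driving movement input, jump, weapon draw and melee.
; Melee activates through the ability component, with combos jumping montage sections.
; Location syncs teleport the pawn on Tick when drift reaches a threshold, while rotation applies immediately, gated by character and montage state.
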(event `EventPossess`
  (params (Pawn :type "Pawn Object Reference"))
  (`self.Possess` Pawn)
  (bind _asbp_aiplayer_character (cast `/Game/Blueprints/Core/BP_AIPlayerCharacter` Pawn))
  (set `self.AIPlayerCharacter` _asbp_aiplayer_character))

(event `PushBcastMove`
  (params (BcastMove :type "BcastMove Structure"))
  (`BcastMoveQueue.Enqueue` (`self.BcastMoveQueue`) BcastMove))

(event `EventRotate`
  (params (Rotation :type "Vector Structure"))
  (`self.ProcRotate` Rotation))

(event `self.ReceiveEndPlay`
  (params (EndPlayReason :type "EEndPlayReason Enum" :default "Destroyed"))
  (bind _bcastmovequeue (`self.BcastMoveQueue`))
  (if (not (`BcastMoveQueue.IsEmpty` _bcastmovequeue))
    (`BcastMoveQueue.Empty` _bcastmovequeue)))

(event `OnLocationSync`
  (params (Location :type "Vector Structure"))
  (set `self.SyncLocation` Location)
  (if (not (`self.IsLocationSync`))
    (set `self.IsLocationSync` true)))

(event `PushBcastAction`
  (params (BcastAction :type "BcastAction Structure"))
  (`BcastActionQueue.Enqueue` (`self.BcastActionQueue`) BcastAction))

(event `self.ReceiveTick`
  (params (DeltaSeconds :type "Float (single-precision)"))
  (bind _aiplayercharacter (`self.AIPlayerCharacter`))
  (`/Engine/EditorBlueprintResources/StandardMacros.IsValid` _aiplayercharacter
    (:`Is Valid`
      (if (`/Game/Blueprints/Core/BP_Character.IsAlive` _aiplayercharacter)
        (`|ExecutionSequence`
          (:`then_0`
            (`self.ProcMove`))
          (:`then_1`
            (`self.Proc Location Sync`))
          (:`then_2`
            (`self.ProcAction`)))))))

(fn `ChangeMove`
  (params (InputMove :type "InputMove Structure"))
  (`self.SetValuesByInputMove` InputMove))

(fn `EndMove`
  (set `self.IsMoving` false))

(fn `Hit`
  (`/Game/Blueprints/Core/BP_Character.EventHit` (`self.AIPlayerCharacter`)))

(fn `InitMove`
  (bind _bcastmovequeue (`self.BcastMoveQueue`))
  (`|ExecutionSequence`
    (:`then_0`
      (if (not (`BcastMoveQueue.IsEmpty` _bcastmovequeue))
        (`BcastMoveQueue.Empty` _bcastmovequeue)))
    (:`then_1`
      (if (`self.IsMoving`)
        (set `self.IsMoving` false)))))

(fn `MoveControlledPawn`
  (bind _returnvalue (`Pawn.GetMovementComponent` (`self.K2_GetPawn`)))
  (`|ExecutionSequence`
    (:`then_0`
      (`PawnMovementComponent.AddInputVector` _returnvalue (* (`self.ForwardVector`) (`self.Forward`)) false))
    (:`then_1`
      (`PawnMovementComponent.AddInputVector` _returnvalue (* (`self.RightVector`) (`self.Right`)) false))))

(fn `Proc Location Sync`
  (bind _returnvalue (`self.K2_GetPawn`))
  (bind _synclocation (`self.SyncLocation`))
  (if (`self.IsLocationSync`)
    (`|ExecutionSequence`
      (:`then_0`
        (if (>= (`KismetMathLibrary.Vector_Distance` (`self.K2_GetActorLocation` _returnvalue) _synclocation) 25.0)
          (`self.K2_SetActorLocation` _returnvalue _synclocation true true)
          (`KismetSystemLibrary.PrintString` "SyncLocation")))
      (:`then_1`
        (set `self.IsLocationSync` false)))))

(fn `ProcAction`
  (bind _aiplayercharacter (`self.AIPlayerCharacter`))
  (bind (_value _returnvalue) (`BcastActionQueue.Dequeue` (`self.BcastActionQueue`)))
  (if _returnvalue
    (`KismetSystemLibrary.PrintString` (`KismetStringLibrary.Concat_StrStr` "BcastInputAction:" (`|GetEnumeratorNameAsString` (`.operation` (break `BcastAction` _value)))))
    (switch `EOpAction` (`.operation` (break `BcastAction` _value))
      (:`Jump`
        (`/Game/Blueprints/Core/BP_PlayerCharacter.EventInputActionJump` _aiplayercharacter))
      (:`DrawWeapon`
        (`/Game/Blueprints/Core/BP_PlayerCharacter.EventInputActionDrawWeapon` _aiplayercharacter))
      (:`MeleeAttack`
        (`self.ProcMeleeAttack` (`.operation` (break `BcastAction` _value)) (`.inputAction` (break `BcastAction` _value)) :!label _label))
      (:`MeleeAttackCombo`
        (goto _label)))))

(fn `ProcMeleeAttack`
  (params (Operation :type "EOpAction Enum" :default "None") (InputAction :type "InputAction Structure"))
  (bind _returnvalue (`|EnumEquality` Operation "MeleeAttackCombo"))
  (bind _aiplayercharacter (`self.AIPlayerCharacter`))
  (bind _returnvalue_2 (`SkeletalMeshComponent.GetAnimInstance` (`Character.Mesh` _aiplayercharacter)))
  (if (or (`/Game/Blueprints/Core/BP_Character.IsUsingSkill` _aiplayercharacter) (`/Game/Blueprints/Core/BP_Character.IsPlayingAction` _aiplayercharacter))
    _
    (elif (`/Game/Blueprints/Core/BP_Character.IsUsingMelee` _aiplayercharacter)
      (if _returnvalue
        (`AnimInstance.Montage_JumpToSection` _returnvalue_2 (`KismetStringLibrary.Conv_StringToName` InputAction_comboSectionName) (`AnimInstance.GetCurrentActiveMontage` _returnvalue_2) :!label _label))
      (else
        (`CharacterAbilityComponent.ActivateAbility` (`/Game/Blueprints/Core/BP_Character.BP_CharacterAbilityComponent` _aiplayercharacter) (make `AbliltyActivationInfo` _aiplayercharacter "MeleeAttack"))
        (if _returnvalue
          (goto _label))))))

(fn `ProcMove`
  (bind (_value _returnvalue) (`BcastMoveQueue.Dequeue` (`self.BcastMoveQueue`)))
  (if _returnvalue
    (`KismetSystemLibrary.PrintString` (`KismetStringLibrary.Concat_StrStr` "BcastMove:" (`|GetEnumeratorNameAsString` (`.operation` (break `BcastMove` _value)))))
    (switch `EOpMove` (`.operation` (break `BcastMove` _value))
      (:`Start`
        (`self.StartMove` (`.inputMove` (break `BcastMove` _value))))
      (:`Change`
        (`self.ChangeMove` (`.inputMove` (break `BcastMove` _value))))
      (:`End`
        (`self.EndMove`))))
  (if (and (`/Game/Blueprints/Core/BP_Character.IsIdle` (`self.AIPlayerCharacter`) false true true true false) (`self.IsMoving`))
    (`self.MoveControlledPawn`)))

(fn `ProcRotate`
  (params (Rotation :type "Vector Structure"))
  (bind _aiplayercharacter (`self.AIPlayerCharacter`))
  (`KismetSystemLibrary.PrintString` "BcastRotate")
  (`/Engine/EditorBlueprintResources/StandardMacros.IsValid` _aiplayercharacter
    (:`Is Valid`
      (if (and (`/Game/Blueprints/Core/BP_Character.IsAlive` _aiplayercharacter) (not (or (`/Game/Blueprints/Core/BP_Character.IsPlayingAction` _aiplayercharacter) (`/Game/Blueprints/Core/BP_Character.IsUsingSkill` _aiplayercharacter))) (`/Game/Blueprints/Core/BP_Character.IsAnyMontagePlaying` _aiplayercharacter))
        (`self.K2_SetActorRotation` _aiplayercharacter (`KismetMathLibrary.Conv_VectorToRotator` Rotation) false)))))

(fn `SetValuesByInputMove`
  (params (InputMove :type "InputMove Structure"))
  (set `self.ForwardVector` InputMove_forwardVector)
  (set `self.RightVector` InputMove_rightVector)
  (set `self.Forward` InputMove_moveForward)
  (set `self.Right` InputMove_moveRight))

(fn `StartMove`
  (params (InputMove :type "InputMove Structure"))
  (`self.SetValuesByInputMove` InputMove)
  (set `self.IsMoving` true))

(fn `UserConstructionScript`
  (`|ExecutionSequence`
    (:`then_0`
      (bind _returnvalue (`|GenericCreateObject` "/Game/Blueprints/Network/Queue/BP_BcastMoveQueue.BP_BcastMoveQueue_C" self))
      (set `self.BcastMoveQueue` _returnvalue))
    (:`then_1`
      (bind _returnvalue_2 (`|GenericCreateObject` "/Game/Blueprints/Network/Queue/BP_BcastActionQueue.BP_BcastActionQueue_C" self))
      (set `self.BcastActionQueue` _returnvalue_2))))