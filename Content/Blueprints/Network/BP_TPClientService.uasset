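; Client network service for a multiplayer game, sending player requests to the server and applying its responses and broadcasts.
; EventGraph wraps login, movement, sync, action, damage, rotation and round-trip-time requests with debug prints.
; RecvEventGraph places the local player on login and spawns or destroys remote players through BP_TPObjectService.
; Remote players act as AI-driven proxies: broadcasts route by user ID to each AIC_Player controller, while local hits go to the player character.
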(event `self.ReceiveBeginPlay`
  (`self.CallBeginPlay`))

(event `self.ReceiveEndPlay`
  (params (EndPlayReason :type "EEndPlayReason Enum" :default "Destroyed"))
  (`self.CallEndPlay` EndPlayReason))

(event `EventReqLogin`
  (params (UserId :type String) (Password :type String))
  (bind _returnvalue (`self.ReqLogin` UserId Password))
  (if _returnvalue
    (`KismetSystemLibrary.PrintString` "ReqLogin")
    (else
      (`KismetSystemLibrary.PrintString` "Fail ReqLogin"))))

(event `EventReqMove`
  (params (Operation :type "EOpMove Enum" :default "Start") (InputMove :type "InputMove Structure"))
  (bind _returnvalue (`self.ReqMove` Operation InputMove))
  (if _returnvalue
    (`KismetSystemLibrary.PrintString` (`KismetStringLibrary.Concat_StrStr` "ReqMove:" (`|GetEnumeratorNameAsString` Operation)))
    (else
      (`KismetSystemLibrary.PrintString` "Fail ReqMove"))))

(event `EventReqMoveSync`
  (params (Location :type "Vector Structure"))
  (bind _returnvalue (`self.ReqMoveSync` Location))
  (if _returnvalue
    (`KismetSystemLibrary.PrintString` "ReqMoveSync")
    (else
      (`KismetSystemLibrary.PrintString` "Fail ReqMoveSync"))))

(event `EventReqRoundTripTime`
  (bind _returnvalue (`self.ReqRoundTripTime`))
  (if _returnvalue
    (`KismetSystemLibrary.PrintString` "ReqRoundTripTime")
    (else
      (`KismetSystemLibrary.PrintString` "Fail ReqRoundTripTime"))))

(event `EventReqAction`
  (params (Operation :type "EOpAction Enum" :default "None") (Pawn :type "Pawn Object Reference"))
  (bind (_returnvalue_roll _returnvalue_pitch _returnvalue_yaw) (`KismetMathLibrary.BreakRotator` (`self.K2_GetActorRotation` Pawn)))
  (bind _returnvalue (`self.ReqAction` Operation (make `InputAction` (`self.K2_GetActorLocation` Pawn) (`KismetMathLibrary.MakeVector` _returnvalue_roll _returnvalue_pitch _returnvalue_yaw))))
  (if _returnvalue
    (`KismetSystemLibrary.PrintString` (`KismetStringLibrary.Concat_StrStr` "ReqAction:" (`|GetEnumeratorNameAsString` Operation)))
    (else
      (`KismetSystemLibrary.PrintString` "Fail ReqAction"))))

(event `EventReqDamage`
  (bind _returnvalue (`self.ReqDamage`))
  (if _returnvalue
    (`KismetSystemLibrary.PrintString` "ReqDamage")
    (else
      (`KismetSystemLibrary.PrintString` "Fail ReqDamage"))))

(event `EventReqRotate`
  (params (Rotation :type "Vector Structure"))
  (bind _returnvalue (`self.ReqRotate` Rotation))
  (if _returnvalue
    (`KismetSystemLibrary.PrintString` "ReqRotate")
    (else
      (`KismetSystemLibrary.PrintString` "Fail ReqRotate"))))

(event `self.K2_RecvCallResLogin`
  (params (objUserList :type "Array of ObjUser Object Reference (by ref)"))
  (bind _tpclientservice (`/Game/Blueprints/Core/BP_FunctionLibrary.GetBPTPClientService`))
  (bind _playercharacter (`/Game/Blueprints/Core/BP_FunctionLibrary.GetBPPlayerCharacter`))
  (`KismetSystemLibrary.PrintString` "로그인에 성공했습니다")
  (for _array_element objUserList
    (bind _returnvalue (`ObjUser.BP_GetUserId` _array_element))
    (if (`KismetStringLibrary.EqualEqual_StrStr` _returnvalue (`self.propUserId`))
      (bind _returnvalue_2 (`ObjUser.BP_GetCompUserTransform` _array_element))
      (bind _returnvalue_3 (`CompUserTransform.BP_GetLocation` _returnvalue_2))
      (`self.K2_SetActorLocation` _playercharacter _returnvalue_3 false false)
      (bind _returnvalue_4 (`CompUserTransform.BP_GetRotation` _returnvalue_2))
      (`self.K2_SetActorRotation` _playercharacter (`KismetMathLibrary.MakeRotator` (.x _returnvalue_4) (.y _returnvalue_4) (.z _returnvalue_4)) false)
      (`/Engine/EditorBlueprintResources/StandardMacros.IsValid` _tpclientservice
        (:`Is Valid`
          (`self.EventReqRoundTripTime` _tpclientservice)))
      (else
        (`/Game/Blueprints/Core/BP_TPObjectService.SpawnNewPlayer` (`/Game/Blueprints/Core/BP_FunctionLibrary.GetBPTPObjectService`) _returnvalue _returnvalue_3 _returnvalue_4)))))

(event `self.K2_RecvCallError`
  (params (message :type String))
  (`KismetSystemLibrary.PrintString` (`KismetStringLibrary.Concat_StrStr` "에러:" message) true true (struct :`R` 1.0 :`B` 0.073311 :`A` 1.0)))

(event `self.K2_RecvCallBcastEnterGameRoom`
  (params (objUser :type "ObjUser Object Reference"))
  (bind _returnvalue (`ObjUser.BP_GetCompUserTransform` objUser))
  (bind _returnvalue_2 (`ObjUser.BP_GetUserId` objUser))
  (`KismetSystemLibrary.PrintString` (`KismetStringLibrary.Concat_StrStr` _returnvalue_2 "님이 입장했습니다"))
  (`/Game/Blueprints/Core/BP_TPObjectService.SpawnNewPlayer` (`/Game/Blueprints/Core/BP_FunctionLibrary.GetBPTPObjectService`) _returnvalue_2 (`CompUserTransform.BP_GetLocation` _returnvalue) (`CompUserTransform.BP_GetRotation` _returnvalue)))

(event `self.K2_RecvCallBcastExitGameRoom`
  (params (userId :type String))
  (`KismetSystemLibrary.PrintString` (`KismetStringLibrary.Concat_StrStr` userId "님이 퇴장했습니다"))
  (`/Game/Blueprints/Core/BP_TPObjectService.DestroyPlayer` (`/Game/Blueprints/Core/BP_FunctionLibrary.GetBPTPObjectService`) userId))

(event `self.K2_RecvCallBcastMove`
  (params (bcastMove :type "BcastMove Structure (by ref)"))
  (bind (_value _returnvalue) (`BlueprintMapLibrary.Map_Find` (`/Game/Blueprints/Core/BP_TPObjectService.PlayerCharacterMap` (`/Game/Blueprints/Core/BP_FunctionLibrary.GetBPTPObjectService`)) (`.userId` (break `BcastMove` bcastMove))))
  (if _returnvalue
    (bind _asaic_player (cast `/Game/Blueprints/AI/AIC_Player` (`AIBlueprintHelperLibrary.GetAIController` _value)))
    (`/Game/Blueprints/AI/AIC_Player.PushBcastMove` _asaic_player bcastMove)))

(event `self.K2_RecvCallBcastLocationSync`
  (params (userId :type String) (location :type "Vector Structure (by ref)"))
  (bind _asaic_player (cast `/Game/Blueprints/AI/AIC_Player` (`AIBlueprintHelperLibrary.GetAIController` (`BlueprintMapLibrary.Map_Find` (`/Game/Blueprints/Core/BP_TPObjectService.PlayerCharacterMap` (`/Game/Blueprints/Core/BP_FunctionLibrary.GetBPTPObjectService`)) userId))))
  (`/Game/Blueprints/AI/AIC_Player.OnLocationSync` _asaic_player location))

(event `self.K2_RecvCallBcastAction`
  (params (bcastAction :type "BcastAction Structure (by ref)"))
  (bind (_value _returnvalue) (`BlueprintMapLibrary.Map_Find` (`/Game/Blueprints/Core/BP_TPObjectService.PlayerCharacterMap` (`/Game/Blueprints/Core/BP_FunctionLibrary.GetBPTPObjectService`)) (`.userId` (break `BcastAction` bcastAction))))
  (if _returnvalue
    (bind _asaic_player (cast `/Game/Blueprints/AI/AIC_Player` (`AIBlueprintHelperLibrary.GetAIController` _value)))
    (`/Game/Blueprints/AI/AIC_Player.PushBcastAction` _asaic_player bcastAction)))

(event `self.K2_RecvCallBcastHit`
  (params (userId :type String))
  (bind _playercharacter (`/Game/Blueprints/Core/BP_FunctionLibrary.GetBPPlayerCharacter`))
  (bind (_value _returnvalue) (`BlueprintMapLibrary.Map_Find` (`/Game/Blueprints/Core/BP_TPObjectService.PlayerCharacterMap` (`/Game/Blueprints/Core/BP_FunctionLibrary.GetBPTPObjectService`)) userId))
  (if _returnvalue
    (bind _asaic_player (cast `/Game/Blueprints/AI/AIC_Player` (`AIBlueprintHelperLibrary.GetAIController` _value)))
    (`/Game/Blueprints/AI/AIC_Player.Hit` _asaic_player)
    (elif (`KismetStringLibrary.EqualEqual_StrStr` userId (`self.propUserId`))
      (`/Engine/EditorBlueprintResources/StandardMacros.IsValid` _playercharacter
        (:`Is Valid`
          (`/Game/Blueprints/Core/BP_Character.EventHit` _playercharacter))))))

(event `self.K2_RecvCallBcastRotate`
  (params (bcastRotate :type "BcastRotate Structure (by ref)"))
  (bind (_value _returnvalue) (`BlueprintMapLibrary.Map_Find` (`/Game/Blueprints/Core/BP_TPObjectService.PlayerCharacterMap` (`/Game/Blueprints/Core/BP_FunctionLibrary.GetBPTPObjectService`)) bcastRotate_userId))
  (if _returnvalue
    (bind _asaic_player (cast `/Game/Blueprints/AI/AIC_Player` (`AIBlueprintHelperLibrary.GetAIController` _value)))
    (`/Game/Blueprints/AI/AIC_Player.EventRotate` _asaic_player bcastRotate_rotation)))

(fn `UserConstructionScript`)