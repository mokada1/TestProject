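; BP_TPClient is a network client Blueprint that connects the game to a server by IP and port.
; ConnectToServer skips if already connected, otherwise calls CreateClientAndConnect, printing Korean status messages for each outcome and returning that call's result.
; Tick calls ProcessPackets every frame to handle packets, and EndPlay passes its reason to CallEndPlay.
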(event `self.ReceiveEndPlay`
  (params (EndPlayReason :type "EEndPlayReason Enum" :default "Destroyed"))
  (`self.CallEndPlay` EndPlayReason))

(event `self.ReceiveTick`
  (params (DeltaSeconds :type "Float (single-precision)"))
  (`self.ProcessPackets`))

(fn `ConnectToServer`
  (params (ServerIp :type String) (ServerPort :type String))
  (returns (Result :type Boolean))
  (if (`self.isConnected`)
    (`KismetSystemLibrary.PrintString` "이미 서버에 접속되어 있습니다")
    (else
      (`KismetSystemLibrary.PrintString` "서버 접속을 시도합니다")
      (bind _returnvalue (`self.CreateClientAndConnect` ServerIp ServerPort))
      (if _returnvalue
        (`KismetSystemLibrary.PrintString` "서버에 접속했습니다")
        (else
          (`KismetSystemLibrary.PrintString` "서버 접속에 실패했습니다")))))
  (return _returnvalue))

(fn `UserConstructionScript`)