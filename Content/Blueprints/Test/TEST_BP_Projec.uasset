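; Test projectile actor that homes in on the player character, with a Niagara effect attached.
; Each Tick it rotates to face the player and steps forward at a constant, frame-rate-independent speed, without sweep.
; Tick also activates the Niagara effect and deactivates it after a short delay, repeatedly.
; Movement is done by setting the transform directly, and the ProjectileMovement reference in the graph is unused.
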(event `self.ReceiveTick`
  (params (DeltaSeconds :type "Float (single-precision)"))
  (bind _playercharacter (`/Game/Blueprints/Core/BP_FunctionLibrary.GetPlayerCharacterBP`))
  (bind _returnvalue (`self.K2_GetActorLocation`))
  (bind _niagara (`self.Niagara`))
  (`|ExecutionSequence`
    (:`then_0`
      (`ActorComponent.Activate` _niagara false)
      (`KismetSystemLibrary.Delay` 0.1)
      (`ActorComponent.Deactivate` _niagara))
    (:`then_1`
      (`/Engine/EditorBlueprintResources/StandardMacros.IsValid` _playercharacter
        (:`Is Valid`
          (`self.K2_SetActorRotation` (`KismetMathLibrary.FindLookAtRotation` _returnvalue (`self.K2_GetActorLocation` _playercharacter)))
          (`self.K2_SetActorLocation` (+ (* (`self.GetActorForwardVector`) (* DeltaSeconds 100.0)) _returnvalue)))))))

(fn `UserConstructionScript`)