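; Blueprint function library of global shortcuts to the project's core objects, plus a location helper.
; Player getters cast player controller 0 to BP_PlayerController and read its PlayerCharacter.
; TP client, client service and object service getters read from BP_GameMode, the client pair through its TPClientPackage.
; GetActorLocationAway rotates an offset by the actor's forward direction and adds it to the actor's location.
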(fn `GetActorLocationAway`
  (params (Actor :type "Actor Object Reference") (`Location Const` :type "Vector Structure"))
  (returns (`Target Location` :type "Vector Structure"))
  (return (+ (`Actor.K2_GetActorLocation` Actor) (`KismetMathLibrary.GreaterGreater_VectorRotator` `Location Const` (`KismetMathLibrary.Conv_VectorToRotator` (`Actor.GetActorForwardVector` Actor))))))

(fn `GetBPPlayerCharacter`
  (returns (PlayerCharacter :type "/Game/Blueprints/Core/BP_PlayerCharacter Object Reference"))
  (bind _playercharacter (`/Game/Blueprints/Core/BP_PlayerController.PlayerCharacter` (`self.GetBPPlayerController` null)))
  (`/Engine/EditorBlueprintResources/StandardMacros.IsValid` _playercharacter
    (:`Is Valid`
      (return _playercharacter))))

(fn `GetBPPlayerController`
  (returns (PlayerController :type "/Game/Blueprints/Core/BP_PlayerController Object Reference"))
  (bind _asbp_player_controller (cast `/Game/Blueprints/Core/BP_PlayerController` (`GameplayStatics.GetPlayerController` null)))
  (return _asbp_player_controller))

(fn `GetBPTPClient`
  (returns (TPClient :type "/Game/Blueprints/Network/BP_TPClient Object Reference"))
  (bind _asbp_game_mode (cast `/Game/Blueprints/Core/BP_GameMode` (`GameplayStatics.GetGameMode` null)))
  (return (`/Game/Blueprints/Network/BP_TPClientPackage.TPClient` (`/Game/Blueprints/Core/BP_GameMode.TPClientPackage` _asbp_game_mode))))

(fn `GetBPTPClientService`
  (returns (TPClientService :type "/Game/Blueprints/Network/BP_TPClientService Object Reference"))
  (bind _asbp_game_mode (cast `/Game/Blueprints/Core/BP_GameMode` (`GameplayStatics.GetGameMode` null)))
  (return (`/Game/Blueprints/Network/BP_TPClientPackage.TPClientService` (`/Game/Blueprints/Core/BP_GameMode.TPClientPackage` _asbp_game_mode))))

(fn `GetBPTPObjectService`
  (params (__WorldContext :type "Object Object Reference"))
  (returns (TPObjectService :type "/Game/Blueprints/Core/BP_TPObjectService Object Reference"))
  (bind _asbp_game_mode (cast `/Game/Blueprints/Core/BP_GameMode` (`GameplayStatics.GetGameMode` null)))
  (return (`/Game/Blueprints/Core/BP_GameMode.TPObjectService` _asbp_game_mode)))