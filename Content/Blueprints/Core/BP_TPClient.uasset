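; BP_TPClient is the Blueprint side of the game's network client, handling server connection and login.
; ConnectToServer stores the server address and user credentials, then calls CreateClientAndConnect and prints the result.
; EventReqLogin sends the stored credentials through ReqLogin, but only when connected.
; RecvCallGameRoomObj reports post-login room entry; all feedback is Korean PrintString messages.
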(event `ConnectToServer`
  (params (ServerIp :type String) (ServerPort :type String) (UserId :type String) (Password :type String))
  (`|ExecutionSequence`
    (:`then_0`
      (set `self.propServerIp` ServerIp)
      (set `self.propServerPort` ServerPort)
      (set `self.propUserId` UserId)
      (set `self.propPassword` Password))
    (:`then_1`
      (`KismetSystemLibrary.PrintString` "서버 접속을 시도합니다")
      (bind _returnvalue (`self.CreateClientAndConnect` (`self.propServerIp`) (`self.propServerPort`)))
      (if _returnvalue
        (`KismetSystemLibrary.PrintString` "서버에 접속했습니다")
        (else
          (`KismetSystemLibrary.PrintString` "서버 접속에 실패했습니다"))))))

(event `EventReqLogin`
  (if (`self.isConnected`)
    (`KismetSystemLibrary.PrintString` "로그인을 시도합니다")
    (`self.ReqLogin` (`self.propUserId`) (`self.propPassword`))))

(event `self.K2_RecvCallGameRoomObj`
  (`KismetSystemLibrary.PrintString` "로그인 성공 후 방에 입장했습니다."))

(fn `UserConstructionScript`)