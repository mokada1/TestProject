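; BP_TPObjectService is an object service that spawns, tracks and destroys player characters by user ID.
; SpawnNewPlayer creates a BP_PlayerCharacter at a given location, always spawning despite collisions, and registers it in PlayerCharacterMap through AddPlayer.
; DestroyPlayer destroys the mapped actor and calls DeletePlayer to remove its entry.
; Each event checks the map first, guarding against duplicate or missing players.
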(event `SpawnNewPlayer`
  (params (UserId :type String) (Location :type "Vector Structure"))
  (if (not (`.ReturnValue` (`BlueprintMapLibrary.Map_Find` (`self.PlayerCharacterMap`) UserId)))
    (bind _returnvalue (`|SpawnActorFromClass` "/Game/Blueprints/Core/BP_PlayerCharacter.BP_PlayerCharacter_C" (`KismetMathLibrary.Conv_VectorToTransform` Location) "AlwaysSpawn" "OverrideRootScale" null null))
    (`self.AddPlayer` UserId _returnvalue)))

(event `AddPlayer`
  (params (UserId :type String) (PlayerCharacter :type "/Game/Blueprints/Core/BP_PlayerCharacter Object Reference"))
  (bind _playercharactermap (`self.PlayerCharacterMap`))
  (if (not (`.ReturnValue` (`BlueprintMapLibrary.Map_Find` _playercharactermap UserId)))
    (`BlueprintMapLibrary.Map_Add` _playercharactermap UserId PlayerCharacter)))

(event `DestroyPlayer`
  (params (UserId :type String))
  (bind (_value _returnvalue) (`BlueprintMapLibrary.Map_Find` (`self.PlayerCharacterMap`) UserId))
  (if _returnvalue
    (`self.K2_DestroyActor` _value)
    (`self.DeletePlayer` UserId)))

(event `DeletePlayer`
  (params (UserId :type String))
  (bind _playercharactermap (`self.PlayerCharacterMap`))
  (if (`.ReturnValue` (`BlueprintMapLibrary.Map_Find` _playercharactermap UserId))
    (`BlueprintMapLibrary.Map_Remove` _playercharactermap UserId)))

(fn `UserConstructionScript`)