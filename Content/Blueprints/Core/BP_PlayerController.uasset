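; Player controller that drives the player character and camera, replicating movement to a server through the BPTP client service.
; Each tick, while the character is alive and not in an action or skill, it either moves camera-relative or, during montages, rotates toward input.
; Movement sends Start/Change/End requests with timer-throttled transform syncs and RTT probes.
; On stopping, it keeps applying the last input for the round-trip time, then force-syncs the transform.
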(event `self.ReceivePossess`
  (params (PossessedPawn :type "Pawn Object Reference"))
  (bind _asbp_player_character (cast `/Game/Blueprints/Core/BP_PlayerCharacter` PossessedPawn))
  (bind _output_get (set `self.PlayerCharacter` _asbp_player_character))
  (set `/Game/Blueprints/Core/BP_Character.Ally` "Player" _output_get))

(event `self.ReceiveTick`
  (params (DeltaSeconds :type "Float (single-precision)"))
  (`self.SetDeltaTimes` DeltaSeconds)
  (`self.UpdateSyncTimer`)
  (`self.Proc Controlling`))

(event `InputAction|Cursor`
  (params (Key :type "Key Structure"))
  ;[1 1 1] Show Mouse Curosr
  (:`Pressed`
    (set `self.bShowMouseCursor` (not (`self.bShowMouseCursor`)))))

(event `InputAxis|Turn`
  (params (AxisValue :type "Float (single-precision)"))
  ;[1 1 1] Camera Turn
  (if (not (`self.bShowMouseCursor`))
    (`self.AddYawInput` AxisValue)))

(event `self.ReceiveBeginPlay`
  (bind _playercameramanager (`self.PlayerCameraManager`))
  ;[1 1 1] Camera Setting
  (set `PlayerCameraManager.ViewPitchMax` 30.0 _playercameramanager)
  (set `PlayerCameraManager.ViewPitchMin` -30.0 _playercameramanager)
  (set `PlayerCameraManager.ViewRollMax` 0.0 _playercameramanager)
  (set `PlayerCameraManager.ViewRollMin` 0.0 _playercameramanager))

(event `InputAxis|LookUp`
  (params (AxisValue :type "Float (single-precision)"))
  ;[1 1 1] Camera Turn
  (if (not (`self.bShowMouseCursor`))
    (`self.AddPitchInput` AxisValue)))

(fn `InitMove`
  (`|ExecutionSequence`
    (:`then_0`
      (set `self.IsMoving` false)
      (set `self.OpMove` "None")
      (set `self.IsDelayMoving` false))
    (:`then_1`
      (set `self.MoveForward` 0.0)
      (set `self.MoveRight` 0.0))
    (:`then_2`
      (set `self.ForwardVector` (0.0 0.0 0.0))
      (set `self.RightVector` (0.0 0.0 0.0)))
    (:`then_3`
      (set `self.LocationSyncTimer` 1.0))))

(fn `IsMoveChange`
  (params (InForwardVector :type "Vector Structure") (InRightVector :type "Vector Structure") (InMoveForward :type "Float (double-precision)") (InMoveRight :type "Float (double-precision)"))
  (returns (Result :type Boolean))
  (return (or (!= (`self.MoveForward`) InMoveForward) (!= (`self.MoveRight`) InMoveRight) (and (!= (`self.ForwardVector`) InForwardVector :`ErrorTolerance` 0.1) (!= InMoveForward 0.0)) (and (!= (`self.RightVector`) InRightVector :`ErrorTolerance` 0.1) (!= InMoveRight 0.0)))))

(fn `IsMoveEnd`
  (params (InMoveForward :type "Float (double-precision)") (InMoveRight :type "Float (double-precision)"))
  (returns (Result :type Boolean))
  (return (and (or (!= (`self.MoveForward`) 0.0) (!= (`self.MoveRight`) 0.0)) (and (== InMoveForward 0.0) (== InMoveRight 0.0)))))

(fn `IsMoveStart`
  (params (InMoveForward :type "Float (double-precision)") (InMoveRight :type "Float (double-precision)"))
  (returns (Result :type Boolean))
  (return (or (and (== (`self.MoveForward`) 0.0) (!= InMoveForward 0.0)) (and (== (`self.MoveRight`) 0.0) (!= InMoveRight 0.0)))))

(fn `MoveCharacter`
  (bind _returnvalue (- (`self.RttMs`) (`self.DeltaMs`)))
  (bind _returnvalue_2 (`PlayerCameraManager.GetCameraRotation` (`self.PlayerCameraManager`)))
  (bind _returnvalue_3 (`KismetMathLibrary.Conv_IntToDouble` (`KismetMathLibrary.Conv_Int64ToInt` (`TPClientService.GetRttMs` (`/Game/Blueprints/Core/BP_FunctionLibrary.GetBPTPClientService`)))))
  (bind _inputmove (make `InputMove` (`KismetMathLibrary.GetForwardVector` _returnvalue_2) (`KismetMathLibrary.GetRightVector` _returnvalue_2) (`self.GetInputAxisValue`) (`self.GetInputAxisValue`)))
  (if (`self.IsDelayMoving`)
    (set `self.RttMs` _returnvalue :!label _label)
    (if (> _returnvalue 0.0)
      (`self.ProcMove` false false false (make `InputMove` (`self.ForwardVector`) (`self.RightVector`) (`self.MoveForward`) (`self.MoveRight`)))
      (else
        (`self.ProcMove` true true true)
        (set `self.IsDelayMoving` false)))
    (else
      (bind _isreqmove (`self.Req Move` _inputmove))
      (if (`|EnumEquality` (`self.OpMove`) "End")
        (if (> _returnvalue_3 (`self.DeltaMs`))
          (set `self.IsDelayMoving` true)
          (set `self.RttMs` _returnvalue_3)
          (goto _label)
          (else
            (`self.ProcMove` true true true _inputmove)))
        (else
          (`self.ProcMove` _isreqmove _isreqmove false _inputmove))))))

(fn `Proc Controlling`
  (bind _playercharacter (`self.PlayerCharacter`))
  (`/Engine/EditorBlueprintResources/StandardMacros.IsValid` _playercharacter
    (:`Is Valid`
      (if (`/Game/Blueprints/Core/BP_PlayerCharacter.IsAlive` _playercharacter)
        (if (or (`/Game/Blueprints/Core/BP_PlayerCharacter.IsPlayingAction` _playercharacter) (`/Game/Blueprints/Core/BP_PlayerCharacter.IsUsingSkill` _playercharacter))
          _
          (elif (`/Game/Blueprints/Core/BP_PlayerCharacter.IsAnyMontagePlaying` _playercharacter)
            (`self.RotateWhileAttacking`)
            (else
              (`self.MoveCharacter`))))))))

(fn `ProcMove`
  (params (IsUpdateMoveValues :type Boolean) (IsSyncTransform :type Boolean :default false) (ForceSyncTransform :type Boolean) (InputMove :type "InputMove Structure"))
  (bind _returnvalue (`self.K2_GetPawn`))
  (`|ExecutionSequence`
    (:`then_0`
      (`Pawn.AddMovementInput` _returnvalue InputMove_forwardVector InputMove_moveForward false))
    (:`then_1`
      (`Pawn.AddMovementInput` _returnvalue InputMove_rightVector InputMove_moveRight false))
    (:`then_2`
      (if IsSyncTransform
        (`self.Req Location Sync` ForceSyncTransform)
        (`self.ReqRotationSync` ForceSyncTransform)
        (`self.ReqRoundTripTime`)))
    (:`then_3`
      (if IsUpdateMoveValues
        (`self.UpdateMoveValues` InputMove_forwardVector InputMove_rightVector InputMove_moveForward InputMove_moveRight)))
    (:`then_4`
      (if (`|EnumInequality` (`self.OpMove`))
        (set `self.OpMove` "None")))))

(fn `Req Location Sync`
  (params (Force :type Boolean))
  (returns (Result :type Boolean))
  (bind _tpclientservice (`/Game/Blueprints/Core/BP_FunctionLibrary.GetBPTPClientService`))
  (`/Engine/EditorBlueprintResources/StandardMacros.IsValid` _tpclientservice
    (:`Is Valid`
      (if (or Force (>= (`self.LocationSyncTimer`) 0.2))
        (`/Game/Blueprints/Network/BP_TPClientService.EventReqLocationSync` _tpclientservice (`self.K2_GetActorLocation` (`self.PlayerCharacter`)))
        (set `self.LocationSyncTimer` 0.0)
        (return true)
        (else
          (return false))))))

(fn `Req Move`
  (params (InputMove :type "InputMove Structure"))
  (returns (IsReqMove :type Boolean))
  (bind (_forwardvector _rightvector _moveforward _moveright) (break `InputMove` InputMove))
  (bind _tpclientservice (`/Game/Blueprints/Core/BP_FunctionLibrary.GetBPTPClientService`))
  (bind _ismoving (`self.IsMoving`))
  (bind _returnvalue (and (not _ismoving) (`self.IsMoveStart` _moveforward _moveright)))
  (bind _returnvalue_2 (and _ismoving (not _returnvalue) (`self.IsMoveEnd` _moveforward _moveright)))
  (`/Engine/EditorBlueprintResources/StandardMacros.IsValid` _tpclientservice
    (:`Is Valid`
      (if _returnvalue
        (set `self.IsMoving` true)
        (set `self.OpMove` "Start")
        (elif _returnvalue_2
          (set `self.IsMoving` false)
          (set `self.OpMove` "End")
          (elif (and _ismoving (not _returnvalue_2) (`self.IsMoveChange` _forwardvector _rightvector _moveforward _moveright))
            (set `self.OpMove` "Change")
            (else
              (return false)))))
      (`/Game/Blueprints/Network/BP_TPClientService.EventReqMove` _tpclientservice (`self.OpMove`) InputMove)
      (return true))))

(fn `ReqRotationSync`
  (params (Force :type Boolean) (IsAttacking :type Boolean) (RotationWhileAttacking :type "Vector Structure"))
  (returns (Result :type Boolean))
  (bind _tpclientservice (`/Game/Blueprints/Core/BP_FunctionLibrary.GetBPTPClientService`))
  (bind (_returnvalue_roll _returnvalue_pitch _returnvalue_yaw) (`KismetMathLibrary.BreakRotator` (`self.K2_GetActorRotation` (`self.PlayerCharacter`))))
  (`/Engine/EditorBlueprintResources/StandardMacros.IsValid` _tpclientservice
    (:`Is Valid`
      (if (or Force (>= (`self.RotationSyncTimer`) 0.2))
        (if IsAttacking
          (`/Game/Blueprints/Network/BP_TPClientService.EventReqRotationSync` _tpclientservice RotationWhileAttacking)
          (else
            (`/Game/Blueprints/Network/BP_TPClientService.EventReqRotationSync` _tpclientservice (`KismetMathLibrary.MakeVector` _returnvalue_roll _returnvalue_pitch _returnvalue_yaw))))
        (set `self.RotationSyncTimer` 0.0)
        (return true)
        (else
          _)))
    (:`Is Not Valid`
      _))
  (return false))

(fn `ReqRoundTripTime`
  (bind _tpclientservice (`/Game/Blueprints/Core/BP_FunctionLibrary.GetBPTPClientService`))
  (`/Engine/EditorBlueprintResources/StandardMacros.IsValid` _tpclientservice
    (:`Is Valid`
      (if (>= (`self.ReqRttTimer`) 0.5)
        (`/Game/Blueprints/Network/BP_TPClientService.EventReqRoundTripTime` _tpclientservice)
        (set `self.ReqRttTimer` 0.0)))))

(fn `RotateWhileAttacking`
  (bind (_returnvalue_roll _returnvalue_pitch _returnvalue_yaw) (`KismetMathLibrary.BreakRotator` (`PlayerCameraManager.GetCameraRotation` (`self.PlayerCameraManager`))))
  (bind _returnvalue (`KismetMathLibrary.MakeVector` (`self.GetInputAxisValue`) (`self.GetInputAxisValue`)))
  (bind _returnvalue_2 (`KismetMathLibrary.NormalizedDeltaRotator` (`KismetMathLibrary.MakeRotFromX` _returnvalue) (`KismetMathLibrary.MakeRotator` 0.0 0.0 (* _returnvalue_yaw -1.0))))
  (bind _returnvalue_3 (`KismetMathLibrary.MakeVector` (.roll _returnvalue_2) (.pitch _returnvalue_2) (.yaw _returnvalue_2)))
  (if (and (>= (`self.RotationSyncTimer`) 0.1) (> (`KismetMathLibrary.VSize` _returnvalue) 0.0))
    (if (!= (`self.RotationWhileAttacking`) _returnvalue_3 :`ErrorTolerance` 0.01)
      (`self.ReqRotationSync` true true _returnvalue_3)
      (`self.K2_SetActorRotation` (`self.K2_GetPawn`) _returnvalue_2 false)
      (set `self.RotationWhileAttacking` _returnvalue_3))))

(fn `SetDeltaTimes`
  (params (DeltaSecs :type "Float (double-precision)"))
  (set `self.DeltaSecs` DeltaSecs)
  (set `self.DeltaMs` (* DeltaSecs 1000.0)))

(fn `UpdateMoveValues`
  (params (InForwardVector :type "Vector Structure") (InRightVector :type "Vector Structure") (InMoveForward :type "Float (double-precision)") (InMoveRight :type "Float (double-precision)"))
  (set `self.MoveForward` InMoveForward)
  (set `self.MoveRight` InMoveRight)
  (set `self.ForwardVector` InForwardVector)
  (set `self.RightVector` InRightVector))

(fn `UpdateSyncTimer`
  (bind _deltasecs (`self.DeltaSecs`))
  (set `self.LocationSyncTimer` (+ _deltasecs (`self.LocationSyncTimer`)))
  (set `self.RotationSyncTimer` (+ _deltasecs (`self.RotationSyncTimer`)))
  (set `self.ReqRttTimer` (+ _deltasecs (`self.ReqRttTimer`))))

(fn `UserConstructionScript`)